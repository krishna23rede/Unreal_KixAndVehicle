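; BP_JetFuelPickup is a pickup that refills jet fuel for the actor that overlaps its mesh.
; On overlap it sends the RefillFuel interface message to that actor without a type check, disables mesh collision and spawns a Niagara pickup effect.
; A WinkOut timeline then drives the mesh's uniform scale and destroys the pickup when it finishes.
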(event `self.PickUpMesh.OnComponentBeginOverlap`
  (params (OverlappedComponent :type "PrimitiveComponent Object Reference") (OtherActor :type "Actor Object Reference") (OtherComp :type "PrimitiveComponent Object Reference") (OtherBodyIndex :type Integer) (bFromSweep :type Boolean) (SweepResult :type "HitResult Structure (by ref)"))
  (message `/Game/Blueprints/Interfaces/BPI_Jetpack.RefillFuel` OtherActor)
  (`PrimitiveComponent.SetCollisionEnabled` (`self.PickUpMesh`) "NoCollision")
  (`NiagaraFunctionLibrary.SpawnSystemAtLocation` "/Game/Assets/Effects/JetFuel/NS_FuelPickup.NS_FuelPickup" (`self.K2_GetActorLocation`))
  (`self.Wink Out`))

(event `Wink Out`
  (bind (_direction _scale) (`Timeline|WinkOut`)
    (:`Update`
      (`SceneComponent.SetWorldScale3D` (`self.PickUpMesh`) (`KismetMathLibrary.MakeVector` _scale _scale _scale)))
    (:`Finished`
      (`self.K2_DestroyActor`))))

(fn `UserConstructionScript`)