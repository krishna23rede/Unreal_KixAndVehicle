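; Player pawn Kix, with a fuel-limited jetpack, interaction input and win/lose end screens.
; Jetpack events toggle two thruster effects and start, loop and stop sounds, while helper functions drain, check and refill fuel, with refills reported to the controller.
; Interaction input messages the stored interactable, and input mapping contexts can be swapped at runtime.
; Win and lose events async-load a centered end-game widget; only losing switches to UI-only input.
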(event `self.ReceiveBeginPlay`
  (bind _asbp_kix_charater_base (cast `/Game/Blueprints/BP_KixCharaterBase` (`self.GetController`)))
  (set `self.PlayerController` _asbp_kix_charater_base))

(event `/Game/Blueprints/Interfaces/BPI_Jetpack.StartJetpack`
  (`ActorComponent.Activate` (`self.Thruster_L`) false)
  (`ActorComponent.Activate` (`self.Thruster_R`) false)
  (`self.StartThrusterSound`))

(event `/Game/Blueprints/Interfaces/BPI_Jetpack.StopJetpack`
  (`ActorComponent.Deactivate` (`self.Thruster_R`))
  (`ActorComponent.Deactivate` (`self.Thruster_L`))
  (`self.StopThrusterSound`))

(event `/Game/Blueprints/Interfaces/BPI_WinLose.WinGame`
  (bind _endgamewidget (`self.EndGameWidget`))
  (`KismetSystemLibrary.PrintString` "WinGame")
  (`|LoadAssetClass` _endgamewidget
    (:`Completed`
      (bind _returnvalue (`|CreateWidget` (`|ConvertAsset` _endgamewidget)))
      (`UserWidget.AddToViewport` _returnvalue 0)
      (`/Game/Blueprints/Widget/WBP_EndGameMenu.SetEndText` _returnvalue "You Win")
      (`UserWidget.SetPositionInViewport` _returnvalue (`self.UpdateLocationToCenter` _returnvalue) true))))

(event `/Game/Blueprints/Interfaces/BPI_WinLose.LoseGame`
  (bind _endgamewidget (`self.EndGameWidget`))
  (bind _playercontroller (`self.PlayerController`))
  (bind _endwidget (`self.EndWidget`))
  (`KismetSystemLibrary.PrintString` "LoseGame" true true (struct :`R` 1.0 :`G` 0.012953 :`A` 1.0))
  (`|LoadAssetClass` _endgamewidget
    (:`Completed`
      (bind _returnvalue (`|CreateWidget` (`|ConvertAsset` _endgamewidget)))
      (bind _output_get (set `self.EndWidget` _returnvalue))
      (`WidgetBlueprintLibrary.SetInputMode_UIOnlyEx` _playercontroller _output_get "LockOnCapture" true)
      (set `PlayerController.bShowMouseCursor` true _playercontroller)
      (`UserWidget.AddToViewport` _endwidget 0)
      (`/Game/Blueprints/Widget/WBP_EndGameMenu.SetEndText` _endwidget "You Lose")
      (`UserWidget.SetPositionInViewport` _endwidget (`self.UpdateLocationToCenter` _endwidget) true))))

(event `/Game/Interafaces/BPI_PlayerInteract.SetInteractable`
  (params (Interactable :type "Actor Object Reference"))
  (set `self.Interactable` Interactable))

(event `EnhancedInput|/Game/Assets/Inputs/IA_Interaction`
  (params (ActionValue :type Boolean) (ElapsedSeconds :type "Float (double-precision)") (TriggeredSeconds :type "Float (double-precision)") (InputAction :type "InputAction Object Reference" :default "/Game/Assets/Inputs/IA_Interaction.IA_Interaction"))
  (:`Started`
    (bind _interactable (`self.Interactable`)
      (:`then`
        (message `/Game/Interafaces/BPI_PlayerInteract.Interact` _interactable self))
      (:`else`))))

(event `/Game/Interafaces/BPI_PlayerInteract.SetInputMappingContext`
  (params (IMC :type "InputMappingContext Object Reference"))
  (bind _playercontroller (`self.PlayerController`))
  (bind _returnvalue (pcsubsystem `EnhancedInputLocalPlayerSubsystem` _playercontroller))
  (`EnhancedInputSubsystemInterface.RemoveMappingContext` _returnvalue (`/Game/Blueprints/BP_KixCharaterBase.PlayerMappingContext` _playercontroller) (struct))
  (`EnhancedInputSubsystemInterface.AddMappingContext` _returnvalue IMC 0 (struct))
  (set `/Game/Blueprints/BP_KixCharaterBase.PlayerMappingContext` IMC (`self.PlayerController`)))

(fn `ConsumeJetFuel`
  (set `self.JetFuel` (`KismetMathLibrary.FClamp` (- (`self.JetFuel`) (* (`self.JetFuelDrainRate`) (`GameplayStatics.GetWorldDeltaSeconds`))) 0.0 (`self.MaxJetFuel`))))

(fn `DrainJetFuel`
  (returns (FuelPercent :type "Float (double-precision)"))
  (`self.ConsumeJetFuel`)
  (return (`KismetMathLibrary.SafeDivide` (`self.JetFuel`) (`self.MaxJetFuel`))))

(fn `GetFuelPercent`
  (returns (`Return Value` :type "Float (double-precision)"))
  (return (`KismetMathLibrary.SafeDivide` (`self.JetFuel`) (`self.MaxJetFuel`))))

(fn `GetInputMappingContext`
  (returns (IMC :type "InputMappingContext Object Reference"))
  (return (`/Game/Blueprints/BP_KixCharaterBase.Mapping Context` (`self.PlayerController`))))

(fn `GetInteractable`
  (returns (Interactable :type "Actor Object Reference"))
  (return null))

(fn `GetMoveInput`
  (returns (InputAction :type "Vector2D Structure"))
  (return (`|GetInputActionValue`)))

(fn `HasFuel`
  (returns (`HasFuel?` :type Boolean))
  (return (> (`self.JetFuel`) 0.0)))

(fn `RefillFuel`
  (set `self.JetFuel` (`self.MaxJetFuel`))
  (bind _playercontroller (`self.PlayerController`)
    (:`then`
      (`/Game/Blueprints/BP_KixCharaterBase.UpdateJetFuel` _playercontroller (`self.MaxJetFuel`))
      (return))
    (:`else`)))

(fn `StartThrusterSound`
  (bind _loopingthrustersound (`self.LoopingThrusterSound`))
  (bind _returnvalue (`GameplayStatics.SpawnSoundAtLocation` "/Game/Assets/Sounds/Thrusters/MS_ThrusterStart.MS_ThrusterStart" (`self.K2_GetActorLocation`) (struct) 1.0 1.0 0.0 "/Game/Assets/Sounds/Thrusters/SA_Thruster.SA_Thruster" null))
  (`AudioComponent.FadeOut` _returnvalue 1.0 0.0 "Linear")
  (`/Engine/EditorBlueprintResources/StandardMacros.IsValid` (`self.LoopingThrusterSound`)
    (:`Is Valid`
      (`AudioComponent.Play` _loopingthrustersound 0.0)
      (`AudioComponent.FadeIn` _loopingthrustersound 0.35 1.0 0.0 "Linear"))
    (:`Is Not Valid`
      (bind _returnvalue_2 (`GameplayStatics.SpawnSoundAttached` "/Game/Assets/Sounds/Thrusters/MS_ThrusterLoop.MS_ThrusterLoop" (`self.CapsuleComponent`) "None" (0.0 0.0 0.0) (struct) "KeepRelativeOffset" false 0.6 1.0 0.0 "/Game/Assets/Sounds/Thrusters/SA_Thruster.SA_Thruster" null))
      (bind _output_get (set `self.LoopingThrusterSound` _returnvalue_2))
      (`AudioComponent.FadeIn` _output_get 0.35 1.0 0.0 "Linear"))))

(fn `StopThrusterSound`
  (bind _loopingthrustersound (`self.LoopingThrusterSound`)
    (:`then`
      (`AudioComponent.Stop` _loopingthrustersound)
      (bind _returnvalue (`GameplayStatics.SpawnSoundAttached` "/Game/Assets/Sounds/Thrusters/MS_ThrusterStop.MS_ThrusterStop" (`self.CapsuleComponent`) "None" (0.0 0.0 0.0) (struct) "KeepRelativeOffset" false 1.0 1.0 0.0 null null))
      (`AudioComponent.FadeOut` _returnvalue 0.35 0.0 "Linear"))
    (:`else`)))

(fn `UpdateLocationToCenter`
  (params (self2 :type "/Game/Blueprints/Widget/WBP_EndGameMenu Object Reference"))
  (returns (ReturnValue :type "Vector2D Structure"))
  (bind (_returnvalue_x _returnvalue_y) (`KismetMathLibrary.BreakVector2D` (`WidgetLayoutLibrary.GetViewportSize`)))
  (bind _sizebox_root (`/Game/Blueprints/Widget/WBP_EndGameMenu.SizeBox_Root` self2))
  (return (`KismetMathLibrary.MakeVector2D` (- (/ _returnvalue_x 2.0) (/ (`SizeBox.WidthOverride` _sizebox_root) 2.0)) (- (/ _returnvalue_y 2.0) (/ (`SizeBox.HeightOverride` _sizebox_root) 2.0)))))

(fn `UserConstructionScript`)