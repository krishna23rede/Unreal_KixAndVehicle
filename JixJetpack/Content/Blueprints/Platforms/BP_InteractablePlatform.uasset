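; BP_InteractablePlatform is an interactable platform Blueprint that is still a stub, with no movement logic.
; On BeginPlay it caches its actor location as InitialPosition and the EndPos component's world location as EndPosition, but neither is used yet.
; Activate and DeActivate only print debug text, both reading "Activated", and Interact returns without doing anything.
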(event `self.ReceiveBeginPlay`
  (set `self.InitialPosition` (`self.K2_GetActorLocation`))
  (set `self.EndPosition` (`SceneComponent.K2_GetComponentLocation` (`self.EndPos`))))

(event `/Game/Blueprints/Interfaces/BPI_Interact.Activate`
  (`KismetSystemLibrary.PrintString` "Activated" true true (struct :`R` 1.0 :`G` 0.037423 :`A` 1.0)))

(event `/Game/Blueprints/Interfaces/BPI_Interact.DeActivate`
  (`KismetSystemLibrary.PrintString` "Activated" true true (struct :`R` 1.0 :`G` 0.037423 :`A` 1.0)))

(fn `Interact`
  (returns (Interactable :type "Actor Object Reference"))
  (return null))

(fn `UserConstructionScript`)