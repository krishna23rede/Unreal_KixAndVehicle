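; BP_PingPongPlatform is a platform that, once activated, moves back and forth between an initial and an end position.
; A timeline drives a vector lerp of the mesh's world location, alternately replaying forward and in reverse on each finish.
; DeActivate only compares the mesh location to EndPos and does not stop the movement.
; Neither position variable is assigned in these graphs.
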(event `/Game/Blueprints/Interfaces/BPI_Interact.Activate`
  (`self.PingPongForward`))

(event `PingPongForward`
  (bind (_direction _float) (`Timeline|Timeline` :!via `PlayFromStart` :!label _label)
    (:`Update`
      (`self.UpdateLerpMovemnt` _float))
    (:`Finished`
      (switch `ETimelineDirection` _direction
        (:`Forward`
          (`self.PingPongReverse`))
        (:`Backward`
          (`self.PingPongForward`))))))

(event `PingPongReverse`
  (goto _label :!via `ReverseFromEnd`))

(event `/Game/Blueprints/Interfaces/BPI_Interact.DeActivate`
  (if (== (`SceneComponent.K2_GetComponentLocation` (`self.PlatFormMesh`)) (`SceneComponent.K2_GetComponentLocation` (`self.EndPos`)) :`ErrorTolerance` 0.1)
    _))

(fn `UpdateLerpMovemnt`
  (params (Alpha :type "Float (single-precision)"))
  (`SceneComponent.K2_SetWorldLocation` (`self.PlatFormMesh`) (`KismetMathLibrary.VLerp` (`self.InitialPosition`) (`self.EndPosition`) Alpha) false false))

(fn `UserConstructionScript`
  (`parent.UserConstructionScript`))